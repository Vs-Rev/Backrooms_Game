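; BP_Menue_3D is a 3D menu actor whose widget component can switch the player's view to other linked menu actors.
; On BeginPlay it binds to the transition dispatcher of its Menue3D_Widget and disables its own collision.
; A dispatched index selects an entry in LinkedMenues, and the view target blends to that actor with easing.
; Each transition moves collision from the current menu to the target, presumably so only the viewed one is interactive.
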(event Custom|TransitionTo
  (params (NewMenue :type BP%20Menue%203D%20Object%20Reference))
  (Collision|SetActorEnableCollision false)
  (Collision|SetActorEnableCollision NewMenue true)
  (Game|Player|SetViewTargetwithBlend (Game|GetPlayerController 0) NewMenue 2.0 "VTBlend_EaseInOut" 2.0 false))

(event Custom|OnTransitionBetweenMenues
  (params (MenueIndex :type Integer))
  (if (Utilities|Array|IsValidIndex (Variables|Default|GetLinkedMenues) MenueIndex)
    (CallFunction|Transitionto (Utilities|Array|Get(acopy) (Variables|Default|GetLinkedMenues) MenueIndex))))

(event EventBeginPlay
  (bind _asmenue_3d_widget (Utilities|Casting|CastToMenue3D_Widget (UserInterface|GetUserWidgetObject (Variables|Default|GetWidget))))
  (EventDispatchers|AssignTransitiontoLinkedMenue _asmenue_3d_widget (delegate Custom|OnTransitionBetweenMenues))
  (Collision|SetActorEnableCollision false))

(fn ConstructionScript)